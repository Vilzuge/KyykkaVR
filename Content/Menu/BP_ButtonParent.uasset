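; BP_ButtonParent is a base VR menu button pressed by touching it with a motion controller fingertip.
; An overlap on its Box sets DisablePress when the other component is the FingerTip of a BP_MotionController, blocking further presses.
; The press does nothing else in this file.
; The construction script copies ButtonText into the TextRender label.
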(event OnComponentBeginOverlap(Box)
  (params (OverlappedComponent :type Primitive%20Component%20Object%20Reference) (OtherActor :type Actor%20Object%20Reference) (OtherComp :type Primitive%20Component%20Object%20Reference) (OtherBodyIndex :type Integer) (bFromSweep :type Boolean) (SweepResult :type Hit%20Result%20Structure%20%28by%20ref%29))
  (if (not (Variables|Default|GetDisablePress))
    (bind _asbp_motion_controller (Utilities|Casting|CastToBP_MotionController OtherActor))
    (if (== (Variables|/Game/VirtualRealityBP/Blueprints/BP_MotionController.BP_MotionController_C|GetFingerTip _asbp_motion_controller) OtherComp)
      (Variables|Default|SetDisablePress true))))

(fn ConstructionScript
  (Rendering|Components|TextRender|SetText (Variables|Default|GetTextRender) (Variables|Default|GetButtonText)))