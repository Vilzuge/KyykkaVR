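; BP_RotateMaila is a grabbable physics actor for motion controllers, with a configurable mass shown as a KG text label.
; The construction script applies the mass override and updates the label.
; Pickup attaches the mesh to the hand through the supplied constraint and stores it.
; Drop breaks that constraint, then after delays launches the mesh upward with a yaw spin impulse and destroys the actor.
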(event EventPickup
  (params (Constraint :type Physics%20Constraint%20Component%20Object%20Reference) (Hand :type Skeletal%20Mesh%20Component%20Object%20Reference))
  (Class|PhysicsConstraintComponent|SetConstrainedComponents Constraint Hand "None" (Variables|Debug|GetStaticMeshComponent) "None")
  (Variables|Default|SetConstraint Constraint))

(event EventDrop
  (bind _constraint (Variables|Default|GetConstraint)
    (:then
      (Class|PhysicsConstraintComponent|BreakConstraint _constraint)
      (Variables|Default|SetConstraint 0)
      (Utilities|FlowControl|Delay 2.0)
      (Physics|AddImpulse (Variables|Debug|GetStaticMeshComponent) "0, 0,350.000000" "None" true)
      (Class|PrimitiveComponent|AddAngularImpulseinDegrees (Variables|Debug|GetStaticMeshComponent) "0.000000,0.000000,40000.000000" "None" true)
      (Utilities|FlowControl|Delay 2.0)
      (Actor|DestroyActor))
    (:else)))

(fn ConstructionScript
  (bind _kg (Variables|Default|GetKG))
  (Class|PrimitiveComponent|SetMassOverrideinKg (Variables|Debug|GetStaticMeshComponent) "None" _kg true)
  (Rendering|Components|TextRender|SetText (Variables|Default|GetTextRender) (Utilities|Text|ToText(String) (Utilities|String|Append (Utilities|String|ToString(Float) _kg) "KG"))))