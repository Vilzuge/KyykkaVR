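; BP_Kyykka is a resettable kyykkä game piece built around a static mesh.
; BeginPlay records the mesh's world location and rotation, and InitialPosRot can capture them again.
; ResetKyykkaPosition moves the mesh back to that saved transform.
; An actor overlap plays a tic sound at the mesh's current location.
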(event EventBeginPlay
  (bind _staticmesh (Variables|Default|GetStaticMesh))
  (Variables|Default|SetOriginalLocation (Transformation|GetWorldLocation _staticmesh))
  (Variables|Default|SetOriginalRotation (Transformation|GetWorldRotation _staticmesh)))

(event EventTick
  (params (DeltaSeconds :type Float%20%28single-precision%29)))

(event Collision|EventActorBeginOverlap
  (params (OtherActor :type Actor%20Object%20Reference))
  (Audio|SpawnSoundatLocation "/Game/SFX/183473__snapper4298__tic.183473__snapper4298__tic" (Transformation|GetWorldLocation (Variables|Default|GetStaticMesh)) "0, 0, 0" 1.0 1.0 0.0 0 0))

(fn ConstructionScript)

(fn ResetKyykkaPosition
  (Transformation|SetWorldLocationAndRotation (Variables|Default|GetStaticMesh) (Variables|Default|GetOriginalLocation) (Variables|Default|GetOriginalRotation) false false))

(fn InitialPosRot
  (bind _staticmesh (Variables|Default|GetStaticMesh))
  (Variables|Default|SetOriginalLocation (Transformation|GetWorldLocation _staticmesh))
  (Variables|Default|SetOriginalRotation (Transformation|GetWorldRotation _staticmesh)))