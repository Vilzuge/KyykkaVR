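; BP_Maila is a physics prop that motion controllers can pick up and drop, with an editable mass shown as a kilogram label.
; Pickup uses the passed physics constraint to join the hand to the static mesh and stores it.
; Drop breaks and clears that stored constraint if it is valid.
; The construction script overrides the mesh's mass with the KG variable and writes that value to the text render.
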(event EventPickup
  (params (Constraint :type Physics%20Constraint%20Component%20Object%20Reference) (Hand :type Skeletal%20Mesh%20Component%20Object%20Reference))
  (Class|PhysicsConstraintComponent|SetConstrainedComponents Constraint Hand "None" (Variables|Debug|GetStaticMeshComponent) "None")
  (Variables|Default|SetConstraint Constraint))

(event EventDrop
  (bind _constraint (Variables|Default|GetConstraint)
    (:then
      (Class|PhysicsConstraintComponent|BreakConstraint _constraint)
      (Variables|Default|SetConstraint 0))
    (:else)))

(fn ConstructionScript
  (bind _kg (Variables|Default|GetKG))
  (Class|PrimitiveComponent|SetMassOverrideinKg (Variables|Debug|GetStaticMeshComponent) "None" _kg true)
  (Rendering|Components|TextRender|SetText (Variables|Default|GetTextRender) (Utilities|Text|ToText(String) (Utilities|String|Append (Utilities|String|ToString(Float) _kg) "KG"))))